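; BP_ChessPlayer is the player pawn for a chess game, handling camera look, piece selection and moves.
; On BeginPlay it registers with BP_ChessGameMode and adds the chess input mapping context.
; On the player's turn, left click traces along the camera's forward vector on separate channels for pieces and move squares, while right click deselects.
; A server move event moves the piece and passes the turn to the other team.
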(event EventBeginPlay
  (bind _returnvalue (PlayerController|LocalPlayerSubsystems|GetEnhancedInputLocalPlayerSubsystem))
  ;[1 1 1] Details for spring arm
  (bind _asbp_chess_game_mode (Utilities|Casting|CastToBP_ChessGameMode (Game|GetGameMode)))
  (Utilities|IsValid _asbp_chess_game_mode
    (:Is%20Valid
      (Default|AddPlayablePawns _asbp_chess_game_mode self)
      (Utilities|IsValid _returnvalue
        (:Is%20Valid
          (Input|AddMappingContext _returnvalue "/Game/Blueprints/Inputs/IMC_ChessInputs.IMC_ChessInputs" 0 "(bIgnoreAllPressedKeysUntilRelease=True,bForceImmediately=False,bNotifyUserSettings=False)"))))))

(event Custom|Server_Move
  (params (Target :type Object%20Object%20Reference) (MovementSquareHit :type Primitive%20Component%20Object%20Reference))
  (Class|BPIChessPiece|Move(Message) Target (Transformation|GetWorldLocation MovementSquareHit))
  (bind _asbp_chess_game_mode (Utilities|Casting|CastToBP_ChessGameMode (Game|GetGameMode)))
  (switch Utilities|FlowControl|Switch|SwitchonChessTeam (Variables|Default|GetTeam)
    (:NewEnumerator0
      (Default|SetCurrentActiveTeamTurn _asbp_chess_game_mode "NewEnumerator1"))
    (:NewEnumerator1
      (Default|SetCurrentActiveTeamTurn _asbp_chess_game_mode "NewEnumerator0"))
    (:NewEnumerator2
      (Development|PrintString "Current team set as none for player"))))

(event Input|EnhancedActionEvents|EnhancedInputActionIA_Look
  (params (ActionValue :type Vector%202D%20Structure) (ElapsedSeconds :type Float%20%28double-precision%29) (TriggeredSeconds :type Float%20%28double-precision%29) (InputAction :type Input%20Action%20Object%20Reference :default "/Game/Blueprints/Inputs/IA_Look.IA_Look"))
  ;[0.1845 0.008568 0.008568 0.5] Camera Look
  (Pawn|Input|AddControllerYawInput (* (.x ActionValue) -1.0))
  (Pawn|Input|AddControllerPitchInput (.y ActionValue)))

(event Input|EnhancedActionEvents|EnhancedInputActionIA_LeftClick
  (params (ActionValue :type Boolean) (ElapsedSeconds :type Float%20%28double-precision%29) (TriggeredSeconds :type Float%20%28double-precision%29) (InputAction :type Input%20Action%20Object%20Reference :default "/Game/Blueprints/Inputs/IA_LeftClick.IA_LeftClick"))
  (bind _asbp_chess_player_controller (Utilities|Casting|CastToBP_ChessPlayerController (Components|GetOwner)))
  (if (Utilities|Enum|Equal(Enum) (Variables|/Game/Blueprints/PlayerController/BP_ChessPlayerController.BP_ChessPlayerController_C|GetCurrentTeamTurn _asbp_chess_player_controller) (Variables|/Game/Blueprints/PlayerController/BP_ChessPlayerController.BP_ChessPlayerController_C|GetChessTeam _asbp_chess_player_controller))
    (bind _outhit_hitactor (Utilities|RaycastUnderMouse "TraceTypeQuery3"))
    (if (Utilities|DoesObjectImplementInterface _outhit_hitactor "/Game/Blueprints/BlueprintInterfaces/BPI_ChessPiece.BPI_ChessPiece_C")
      (if (not (== (Variables|Default|GetLastSelectedPiece) _outhit_hitactor))
        (bind _lastselectedpiece (Variables|Default|GetLastSelectedPiece) ; Check if there was a prior piece selected
          (:then
            (Class|BPIChessPiece|DeSelect(Message) _lastselectedpiece)
            (bind _asbp_base_chess_piece (Utilities|Casting|CastToBP_BaseChessPiece _outhit_hitactor))
            (if (Utilities|Enum|Equal(Enum) (Variables|/Game/Blueprints/Actors/BP_BaseChessPiece.BP_BaseChessPiece_C|GetTeam _asbp_base_chess_piece) (Variables|Default|GetTeam))
              (Class|BPIChessPiece|DeSelect(Message) (Variables|Default|GetLastSelectedPiece))
              (bind _output_get (Variables|Default|SetLastSelectedPiece _asbp_base_chess_piece))
              (Class|BPIChessPiece|Select(Message) _output_get)
              (else
                (bind _out_hit_hit_component (Utilities|RaycastUnderMouse "TraceTypeQuery4"))
                (Utilities|IsValid _out_hit_hit_component
                  (:Is%20Valid
                    (Utilities|IsValid (Variables|Default|GetLastSelectedPiece)
                      (:Is%20Valid
                        (CallFunction|ServerMove (Variables|Default|GetLastSelectedPiece) _out_hit_hit_component)
                        (Class|BPIChessPiece|DeSelect(Message) (stale _lastselectedpiece_2) :!label _label)
                        (Variables|Default|SetLastSelectedPiece 0))))))))
          (:else
            (bind _asbp_base_chess_piece_2 (Utilities|Casting|CastToBP_BaseChessPiece _outhit_hitactor))
            (if (Utilities|Enum|Equal(Enum) (Variables|/Game/Blueprints/Actors/BP_BaseChessPiece.BP_BaseChessPiece_C|GetTeam _asbp_base_chess_piece_2) (Variables|Default|GetTeam))
              (bind _output_get_2 (Variables|Default|SetLastSelectedPiece _outhit_hitactor))
              (bind _asbp_base_chess_piece_3 (Utilities|Casting|CastToBP_BaseChessPiece _output_get_2))
              (Default|Select _asbp_base_chess_piece_3)
              (else
                (Development|PrintString "Not one of your pieces"))))))
      (else
        (bind _lastselectedpiece_2 (Variables|Default|GetLastSelectedPiece)
          (:then
            (bind _out_hit_hit_component_2 (Utilities|RaycastUnderMouse "TraceTypeQuery4"))
            (Utilities|IsValid _out_hit_hit_component_2
              (:Is%20Valid
                (CallFunction|ServerMove (Variables|Default|GetLastSelectedPiece) _out_hit_hit_component_2)
                (goto _label))
              (:Is%20Not%20Valid
                (goto _label))))
          (:else))))))

(event Input|EnhancedActionEvents|EnhancedInputActionIA_LeftClickRelease
  (params (ActionValue :type Boolean) (ElapsedSeconds :type Float%20%28double-precision%29) (TriggeredSeconds :type Float%20%28double-precision%29) (InputAction :type Input%20Action%20Object%20Reference :default "/Game/Blueprints/Inputs/IA_LeftClickRelease.IA_LeftClickRelease")))

(event Input|EnhancedActionEvents|EnhancedInputActionIA_RightClick
  (params (ActionValue :type Boolean) (ElapsedSeconds :type Float%20%28double-precision%29) (TriggeredSeconds :type Float%20%28double-precision%29) (InputAction :type Input%20Action%20Object%20Reference :default "/Game/Blueprints/Inputs/IA_RightClick.IA_RightClick"))
  (bind _lastselectedpiece (Variables|Default|GetLastSelectedPiece)
    (:then
      (Class|BPIChessPiece|DeSelect(Message) _lastselectedpiece)
      (Variables|Default|SetLastSelectedPiece 0))
    (:else)))

(fn ConstructionScript)