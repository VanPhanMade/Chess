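; Chess game mode for a two-player match that assigns colours, runs turns and detects checkmate.
; Once two players join, PostLogin randomly possesses the registered pawns and starts White's turn.
; Each turn change updates both controllers, tests the active king for check, and totals valid moves, only printing on checkmate.
; It also routes promotion and registers kings and pieces, though black pieces are written into the white array.
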(event Custom|AddPlayablePawns
  (params (PlayablePawn :type BP%20Chess%20Player%20Object%20Reference%20%28by%20ref%29))
  ;[0.3325 0.01681 0.016 0.5] Addings playable pawn instance so gamemode can reference them
  (if (not (Utilities|Array|ContainsItem (Variables|Default|GetPlayablePawns) PlayablePawn))
    (Utilities|Array|Add (Variables|Default|GetPlayablePawns) PlayablePawn)))

(event Custom|SetCurrentActiveTeamTurn
  (params (TeamToTakeTurn :type ChessTeam%20Enum :default "NewEnumerator0"))
  (bind _playerwhite (Variables|Default|GetPlayerWhite))
  (bind _playerblack (Variables|Default|GetPlayerBlack))
  ;[0.5333 0.02122 0.02122 0.5] Also contains checking for checkmate once a player switch occurs
  (Variables|Default|SetNumberOfValidMoves 0.0)
  (if (Utilities|Enum|NotEqual(Enum) TeamToTakeTurn "NewEnumerator2")
    (bind _output_get (Variables|/Game/Blueprints/PlayerController/BP_ChessPlayerController.BP_ChessPlayerController_C|SetCurrentTeamTurn (Variables|Default|GetPlayerWhite) TeamToTakeTurn))
    (Variables|/Game/Blueprints/PlayerController/BP_ChessPlayerController.BP_ChessPlayerController_C|SetCurrentTeamTurn (Variables|Default|GetPlayerBlack) _output_get)
    (Utilities|FlowControl|Delay 0.2)
    (Default|UpdateUI (Variables|Default|GetPlayerWhite) false)
    (Default|UpdateUI (Variables|Default|GetPlayerBlack) false)
    (switch Utilities|FlowControl|Switch|SwitchonChessTeam TeamToTakeTurn
      (:NewEnumerator0
        (bind _isincheck (Default|CalculateinCheck (Variables|Default|GetBlackKing)))
        (bind _asbp_chess_player (Utilities|Casting|CastToBP_ChessPlayer (Pawn|GetControlledPawn _playerblack)))
        (bind _output_get_2 (Variables|/Game/Blueprints/Pawn/BP_ChessPlayer.BP_ChessPlayer_C|SetInCheck _asbp_chess_player _isincheck))
        (if _output_get_2
          (bind _array_element (Utilities|Array|ForEachLoopwithBreak (Variables|Default|GetAllBlackPieces))
            (:LoopBody
              (bind _validmovesincheck (Default|ReturnNumberOfValidMoves _array_element))
              (Variables|Default|SetNumberOfValidMoves (+ _validmovesincheck (Variables|Default|GetNumberOfValidMoves))))
            (:Completed
              (if (> (Variables|Default|GetNumberOfValidMoves) 0.0)
                (Default|UpdateUI _playerblack _output_get_2 :!label _label)
                (else
                  (Development|PrintString "In Checkmate" :!label _label_2)))))
          (else
            (goto _label))))
      (:NewEnumerator1
        (bind _isincheck_2 (Default|CalculateinCheck (Variables|Default|GetWhiteKing)))
        (bind _asbp_chess_player_2 (Utilities|Casting|CastToBP_ChessPlayer (Pawn|GetControlledPawn _playerwhite)))
        (bind _output_get_3 (Variables|/Game/Blueprints/Pawn/BP_ChessPlayer.BP_ChessPlayer_C|SetInCheck _asbp_chess_player_2 _isincheck_2))
        (if _output_get_3
          (bind _array_element_2 (Utilities|Array|ForEachLoopwithBreak (Variables|Default|GetAllWhitePieces))
            (:LoopBody
              (bind _validmovesincheck_2 (Default|ReturnNumberOfValidMoves _array_element_2))
              (Variables|Default|SetNumberOfValidMoves (+ _validmovesincheck_2 (Variables|Default|GetNumberOfValidMoves))))
            (:Completed
              (if (> (Variables|Default|GetNumberOfValidMoves) 0.0)
                (Default|UpdateUI _playerwhite _output_get_3 :!label _label_3)
                (else
                  (goto _label_2)))))
          (else
            (goto _label_3)))))))

(event Custom|AddKings
  (params (King :type BP%20King%20Object%20Reference))
  (if (not (or (== (Variables|Default|GetBlackKing) King) (== King (Variables|Default|GetWhiteKing))))
    (switch Utilities|FlowControl|Switch|SwitchonChessTeam (Variables|/Game/Blueprints/Actors/BP_BaseChessPiece.BP_BaseChessPiece_C|GetTeam King)
      (:NewEnumerator0
        (Variables|Default|SetBlackKing King))
      (:NewEnumerator1
        (Variables|Default|SetWhiteKing King))
      (:NewEnumerator2
        (Development|PrintString "King missing team role")))))

(event Custom|AddTeamPieces
  (params (Piece :type BP%20Base%20Chess%20Piece%20Object%20Reference))
  (switch Utilities|FlowControl|Switch|SwitchonChessTeam (Variables|/Game/Blueprints/Actors/BP_BaseChessPiece.BP_BaseChessPiece_C|GetTeam Piece)
    (:NewEnumerator0
      (if (not (Utilities|Array|ContainsItem (Variables|Default|GetAllBlackPieces) Piece))
        (Utilities|Array|Add (Variables|Default|GetAllWhitePieces) Piece)))
    (:NewEnumerator1
      (if (not (Utilities|Array|ContainsItem (Variables|Default|GetAllWhitePieces) Piece))
        (Utilities|Array|Add (Variables|Default|GetAllWhitePieces) Piece)))))

(event Custom|TogglePawnPromotion
  (params (Team :type ChessTeam%20Enum :default "NewEnumerator0") (PawnToPromote :type BP%20Pawn%20Object%20Reference))
  (switch Utilities|FlowControl|Switch|SwitchonChessTeam Team
    (:NewEnumerator0
      (Default|TogglePromotionSelection (Variables|Default|GetPlayerBlack) PawnToPromote)
      (Development|PrintString "Promotion Black" true true "(R=0.000000,G=0.660000,B=1.000000,A=1.000000)" 1.0))
    (:NewEnumerator1
      (Default|TogglePromotionSelection (Variables|Default|GetPlayerWhite) PawnToPromote)
      (Development|PrintString "Promotion White" true true "(R=0.000000,G=0.660000,B=1.000000,A=1.000000)" 1.0))
    (:NewEnumerator2
      (Development|PrintString "Missing Team"))))

(event Custom|ReplacePawn
  (params (NewPiece :type BP%20Base%20Chess%20Piece%20Object%20Reference) (Team :type ChessTeam%20Enum :default "NewEnumerator0"))
  (bind _allwhitepieces (Variables|Default|GetAllWhitePieces))
  (switch Utilities|FlowControl|Switch|SwitchonChessTeam Team
    (:NewEnumerator0
      (bind (_array_element _array_index) (Utilities|Array|ForEachLoopwithBreak (Variables|Default|GetAllBlackPieces) :!label _label)
        (:LoopBody
          (Utilities|IsValid _array_element
            (:Is%20Not%20Valid
              (Utilities|Array|Insert _allwhitepieces NewPiece _array_index)
              (goto _label Break))))
        (:Completed
          _)))
    (:NewEnumerator1
      (bind (_array_element_2 _array_index_2) (Utilities|Array|ForEachLoopwithBreak _allwhitepieces :!label _label_2)
        (:LoopBody
          (Utilities|IsValid _array_element_2
            (:Is%20Not%20Valid
              (Utilities|Array|Insert _allwhitepieces NewPiece _array_index_2)
              (goto _label_2 Break))))
        (:Completed
          _))))
  (switch Utilities|FlowControl|Switch|SwitchonChessTeam Team
    (:NewEnumerator0
      (CallFunction|SetCurrentActiveTeamTurn "NewEnumerator1"))
    (:NewEnumerator1
      (CallFunction|SetCurrentActiveTeamTurn "NewEnumerator0"))))

(event EventPostLogin
  (params (NewPlayer :type Player%20Controller%20Object%20Reference))
  (bind _players (Variables|Default|GetPlayers))
  (bind _players_2 (Variables|Default|GetPlayers))
  (bind _playablepawns (Variables|Default|GetPlayablePawns))
  (bind _players_3 (Variables|Default|GetPlayers))
  (bind _playablepawns_2 (Variables|Default|GetPlayablePawns))
  (bind _players_4 (Variables|Default|GetPlayers))
  (bind _output (Utilities|Array|Get(acopy) _players))
  (bind _output_2 (Utilities|Array|Get(acopy) _players_2))
  ;[0.1845 0.007499 0.007499 0.5] Wait for 2 players to join, then assign a random color between two players
  (Utilities|Array|Add (Variables|Default|GetPlayers) NewPlayer)
  (bind _asbp_chess_player_controller (Utilities|Casting|CastToBP_ChessPlayerController NewPlayer))
  (Utilities|IsValid _asbp_chess_player_controller
    (:Is%20Valid
      (Utilities|FlowControl|Delay 0.5)
      (for _array_element (Variables|Default|GetPlayers)
        (bind _asbp_chess_player_controller_2 (Utilities|Casting|CastToBP_ChessPlayerController _array_element))
        (bind _returnvalue (Class|GameModeBase|GetNumPlayers))
        (Default|PlayerJoined _asbp_chess_player_controller_2 _returnvalue)
        (if (== _returnvalue 2) :!label _label
          (switch int (Math|Random|RandomInteger 3)
            (:Default
              (goto _label))
            (:1
              ;[1 1 1] Player 0 gets Pawn 0, Player 1 gets Pawn 1
              (Pawn|Possess (Utilities|Array|Get(acopy) _players_4) (Utilities|Array|Get(acopy) _playablepawns_2))
              (Pawn|Possess (Utilities|Array|Get(acopy) _players_4 1) (Utilities|Array|Get(acopy) _playablepawns_2 1))
              ;[1 1 1] Setting up respective player
              (switch Utilities|FlowControl|Switch|SwitchonChessTeam (Variables|/Game/Blueprints/Pawn/BP_ChessPlayer.BP_ChessPlayer_C|GetTeam (Utilities|Array|Get(acopy) (Variables|Default|GetPlayablePawns)))
                (:NewEnumerator0
                  (bind _asbp_chess_player_controller_3 (Utilities|Casting|CastToBP_ChessPlayerController _output_2))
                  (Variables|Default|SetPlayerBlack _asbp_chess_player_controller_3)
                  (bind _asbp_chess_player_controller_4 (Utilities|Casting|CastToBP_ChessPlayerController (Utilities|Array|Get(acopy) (Variables|Default|GetPlayers) 1)))
                  (Variables|Default|SetPlayerWhite _asbp_chess_player_controller_4)
                  ;[1 1 1] Setting values on controller so UI and game mechanics update accordingly
                  (Variables|/Game/Blueprints/PlayerController/BP_ChessPlayerController.BP_ChessPlayerController_C|SetChessTeam (Variables|Default|GetPlayerWhite) "NewEnumerator1" :!label _label_2)
                  (Variables|/Game/Blueprints/PlayerController/BP_ChessPlayerController.BP_ChessPlayerController_C|SetChessTeam (Variables|Default|GetPlayerBlack) "NewEnumerator0")
                  (CallFunction|SetCurrentActiveTeamTurn "NewEnumerator1"))
                (:NewEnumerator1
                  (bind _asbp_chess_player_controller_5 (Utilities|Casting|CastToBP_ChessPlayerController _output_2))
                  (Variables|Default|SetPlayerWhite _asbp_chess_player_controller_5)
                  (bind _asbp_chess_player_controller_6 (Utilities|Casting|CastToBP_ChessPlayerController (Utilities|Array|Get(acopy) (Variables|Default|GetPlayers) 1)))
                  (Variables|Default|SetPlayerBlack _asbp_chess_player_controller_6)
                  (goto _label_2))
                (:NewEnumerator2
                  (Development|PrintString "Got none for team setting!"))))
            (:2
              ;[1 1 1] Player 0 gets Pawn 1 Player 1 gets Pawn 0
              (Pawn|Possess (Utilities|Array|Get(acopy) _players_3) (Utilities|Array|Get(acopy) _playablepawns 1))
              (Pawn|Possess (Utilities|Array|Get(acopy) _players_3 1) (Utilities|Array|Get(acopy) _playablepawns))
              (switch Utilities|FlowControl|Switch|SwitchonChessTeam (Variables|/Game/Blueprints/Pawn/BP_ChessPlayer.BP_ChessPlayer_C|GetTeam (Utilities|Array|Get(acopy) (Variables|Default|GetPlayablePawns) 1))
                (:NewEnumerator0
                  (bind _asbp_chess_player_controller_7 (Utilities|Casting|CastToBP_ChessPlayerController _output))
                  (Variables|Default|SetPlayerBlack _asbp_chess_player_controller_7)
                  (bind _asbp_chess_player_controller_8 (Utilities|Casting|CastToBP_ChessPlayerController (Utilities|Array|Get(acopy) (Variables|Default|GetPlayers) 1)))
                  (Variables|Default|SetPlayerWhite _asbp_chess_player_controller_8)
                  (goto _label_2))
                (:NewEnumerator1
                  (bind _asbp_chess_player_controller_9 (Utilities|Casting|CastToBP_ChessPlayerController _output))
                  (Variables|Default|SetPlayerWhite _asbp_chess_player_controller_9)
                  (bind _asbp_chess_player_controller_10 (Utilities|Casting|CastToBP_ChessPlayerController (Utilities|Array|Get(acopy) (Variables|Default|GetPlayers) 1)))
                  (Variables|Default|SetPlayerBlack _asbp_chess_player_controller_10)
                  (goto _label_2))
                (:NewEnumerator2
                  (Development|PrintString "Got none for team setting!"))))))))))

(fn ConstructionScript)

(fn GetKingPosition
  (params (Team :type ChessTeam%20Enum :default "NewEnumerator0"))
  (switch Utilities|FlowControl|Switch|SwitchonChessTeam Team
    (:NewEnumerator0
      (bind _blackking (Variables|Default|GetBlackKing)
        (:then
          (LocalVariables|SetKingPos (Transformation|GetActorLocation _blackking)))
        (:else)))
    (:NewEnumerator1
      (bind _whiteking (Variables|Default|GetWhiteKing)
        (:then
          (LocalVariables|SetKingPos (Transformation|GetActorLocation _whiteking)))
        (:else))))
  (return (LocalVariables|GetKingPos)))