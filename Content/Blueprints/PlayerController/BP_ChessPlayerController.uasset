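; Player controller for a multiplayer chess game that manages the local player's input mapping and in-game UI.
; On BeginPlay it adds the chess mapping context and, for a BP_Observer pawn, creates WBP_InGameUI.
; Player-count events switch waiting, opponent-found and crosshair displays, while RepNotifies on team and current turn update turn text.
; It also shows check status and opens pawn promotion selection in UI-only input; CheckmateUI is an empty stub.
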(event Custom|PlayerJoined
  (params (NumberOfPlayers :type Integer))
  (bind _ingameui (Variables|Default|GetInGameUI))
  (switch int NumberOfPlayers
    (:1
      (Default|ToggleWaiting _ingameui))
    (:2
      (Default|ToggleOpponentFound _ingameui)
      (Utilities|FlowControl|Delay 1.5)
      (Default|ToggleCrosshair _ingameui))))

(event EventBeginPlay
  (bind _returnvalue (PlayerController|LocalPlayerSubsystems|GetEnhancedInputLocalPlayerSubsystem))
  (Utilities|IsValid _returnvalue
    (:Is%20Valid
      (Input|AddMappingContext _returnvalue "/Game/Blueprints/Inputs/IMC_ChessInputs.IMC_ChessInputs" 0 "(bIgnoreAllPressedKeysUntilRelease=True,bForceImmediately=False,bNotifyUserSettings=False)")
      (bind _asbp_observer (Utilities|Casting|CastToBP_Observer (Pawn|GetControlledPawn)))
      (Utilities|IsValid _asbp_observer
        (:Is%20Valid
          (Variables|Default|SetInGameUI (Variables|/Game/Blueprints/Pawn/BP_Observer.BP_Observer_C|GetInGameUI_Ref _asbp_observer))
          (bind _returnvalue_2 (UserInterface|CreateWidget "/Game/Blueprints/Widgets/HUDs/WBP_InGameUI.WBP_InGameUI_C" (Game|GetPlayerController 0)))
          (UserInterface|Viewport|AddtoViewport _returnvalue_2 0)
          (Variables|Default|SetInGameUI _returnvalue_2))))))

(fn ConstructionScript)

(fn ToggleWaiting
  (Default|ToggleWaiting (Variables|Default|GetInGameUI)))

(fn ToggleChoosingSide
  (Default|ToggleOpponentFound (Variables|Default|GetInGameUI)))

(fn OnRepChessTeam
  (bind _ingameui (Variables|Default|GetInGameUI))
  (Variables|Default|GetInGameUI
    (:then
      (switch Utilities|FlowControl|Switch|SwitchonChessTeam (Variables|Default|GetChessTeam)
        (:NewEnumerator0
          (Default|YourTurnText _ingameui false))
        (:NewEnumerator1
          (Default|YourTurnText _ingameui true))))
    (:else)))

(fn OnRepCurrentTeamTurn
  (bind _ingameui (Variables|Default|GetInGameUI)
    (:then
      (Default|YourTurnText _ingameui (Utilities|Enum|Equal(Enum) (Variables|Default|GetChessTeam) (Variables|Default|GetCurrentTeamTurn))))
    (:else)))

(fn UpdateUI
  (params (IsInCheck :type Boolean))
  (bind _ingameui (Variables|Default|GetInGameUI)
    (:then
      (Default|YourTurnText _ingameui (Utilities|Enum|Equal(Enum) (Variables|Default|GetChessTeam) (Variables|Default|GetCurrentTeamTurn)))
      (Default|InCheckText _ingameui IsInCheck))
    (:else)))

(fn TogglePromotionSelection
  (params (PawnToPromote :type BP%20Pawn%20Object%20Reference))
  (bind _self self)
  (bind _ingameui (Variables|Default|GetInGameUI))
  (Utilities|IsValid PawnToPromote
    (:Is%20Valid
      (Variables|Default|SetPawnToPromote PawnToPromote)
      (Utilities|IsValid _ingameui
        (:Is%20Valid
          (Default|TogglePiecesSelection _ingameui)
          (Input|SetInputModeUIOnly _self _ingameui "DoNotLock" false)
          (Variables|Default|SetbShowMouseCursor _self true))))))

(fn CheckmateUI
  (params (WonGame :type Boolean) (DrawGame :type Boolean)))