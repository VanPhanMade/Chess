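; BP_Knight is the chess knight, with eight move-square components for its L-shaped jumps.
; ShowValidMoves runs the CalculateValidMoves macro on each square, tracing down to confirm the board and up to detect an occupant.
; Squares that are empty or hold an opposing BP_BaseChessPiece become visible and collidable.
; DeSelect hides those squares, disables their collision and sets the piece's outline overlay to clear.
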(event EventDeSelect
  (Rendering|SetVisibility (Variables|Default|GetLeftForward) false false)
  (Rendering|Material|SetOverlayMaterial (Variables|Default|GetChessPiece) "/Game/Art/Materials/M_OutlineClear.M_OutlineClear" :!class /Script/Engine.MeshComponent)
  (Collision|SetCollisionEnabled (Variables|Default|GetLeftForward) "NoCollision"))

(event EventShowValidMoves
  (Utilities|CalculateValidMoves (Variables|Default|GetLeftForward)
    (:Out
      (Utilities|CalculateValidMoves (Variables|Default|GetBackLeft)
        (:Out
          (Utilities|CalculateValidMoves (Variables|Default|GetRightBack)
            (:Out
              (Utilities|CalculateValidMoves (Variables|Default|GetBackRight)
                (:Out
                  (Utilities|CalculateValidMoves (Variables|Default|GetLeftBack)
                    (:Out
                      (Utilities|CalculateValidMoves (Variables|Default|GetRightForward)
                        (:Out
                          (Utilities|CalculateValidMoves (Variables|Default|GetForwardLeft)
                            (:Out
                              (Utilities|CalculateValidMoves (Variables|Default|GetForwardRight)))))))))))))))))

(fn ConstructionScript
  (|CallParentFunction))