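; Base chess piece actor that handles selection, movement and capture, registering with BP_ChessGameMode and caching its team's king.
; Selecting applies an outline overlay and shows valid moves unless pinned; show and hide are placeholder prints here.
; IsPinned line-traces away from the king for an enemy queen, rook or bishop.
; Move traces upward to destroy any occupant, teleports the piece and plays a board-hit event.
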(event Custom|Server_Select
  (Variables|Default|SetSelected true)
  (Rendering|Material|SetOverlayMaterial (Variables|Default|GetChessPiece) "/Game/Art/Materials/M_Outline.M_Outline" :!class /Script/Engine.MeshComponent)
  (bind _ispinned (CallFunction|IsPinned))
  (if (not _ispinned)
    (CallFunction|ShowValidMoves)))

(event Custom|Server_Deselect
  (Variables|Default|SetSelected false)
  (Rendering|Material|SetOverlayMaterial (Variables|Default|GetChessPiece) "/Game/Art/Materials/M_OutlineClear.M_OutlineClear" :!class /Script/Engine.MeshComponent)
  (CallFunction|HideValidMoves))

(event EventBeginPlay
  (bind _asbp_chess_game_mode (Utilities|Casting|CastToBP_ChessGameMode (Game|GetGameMode)))
  (Utilities|FlowControl|Delay 0.5)
  (Default|AddTeamPieces _asbp_chess_game_mode self)
  (switch Utilities|FlowControl|Switch|SwitchonChessTeam (Variables|Default|GetTeam)
    (:NewEnumerator0
      (Variables|Default|SetPieceKing (Variables|/Game/Blueprints/GameMode/BP_ChessGameMode.BP_ChessGameMode_C|GetBlackKing _asbp_chess_game_mode)))
    (:NewEnumerator1
      (Variables|Default|SetPieceKing (Variables|/Game/Blueprints/GameMode/BP_ChessGameMode.BP_ChessGameMode_C|GetWhiteKing _asbp_chess_game_mode)))))

(event EventHideValidMoves
  (Development|PrintString "Base Hide"))

(event EventSelect
  (Variables|Default|SetSelected true)
  (Rendering|Material|SetOverlayMaterial (Variables|Default|GetChessPiece) "/Game/Art/Materials/M_Outline.M_Outline" :!class /Script/Engine.MeshComponent)
  (bind _ispinned (CallFunction|IsPinned))
  (if (not _ispinned)
    (CallFunction|ShowValidMoves)))

(event EventDeSelect
  (Variables|Default|SetSelected false)
  (Rendering|Material|SetOverlayMaterial (Variables|Default|GetChessPiece) "/Game/Art/Materials/M_OutlineClear.M_OutlineClear" :!class /Script/Engine.MeshComponent)
  (CallFunction|HideValidMoves))

(event EventShowValidMoves
  (Development|PrintString "Base Show"))

(event EventMove
  (params (NewLocation :type Vector :default "0, 0, 0"))
  (bind _output_get (Variables|Default|SetNewLocation NewLocation))
  (bind (_outhit _returnvalue) (Collision|LineTraceByChannel _output_get (+ _output_get (* (Math|Vector|VectorUp) 1e+02)) "TraceTypeQuery3" false 0 "None"))
  (if _returnvalue ; Destroy pieces on take locations
    (Actor|DestroyActor (.hitactor _outhit)))
  (Transformation|SetActorLocation (Variables|Default|GetNewLocation) false false)
  (Variables|Default|SetMoved true)
  (Class|FMODBlueprintStatics|PlayEventatLocation "/Game/FMOD/Events/SFX/PieceHitBoard.PieceHitBoard" (Math|Transform|MakeTransform (Transformation|GetActorLocation) "0, 0, 0" "1.000000,1.000000,1.000000")))

(fn ConstructionScript)

(fn OnRepSelected)

(fn IsPinned
  (bind _returnvalue (Transformation|GetActorLocation))
  (bind _asbp_chess_game_mode (Utilities|Casting|CastToBP_ChessGameMode (Game|GetGameMode)))
  (Utilities|IsValid _asbp_chess_game_mode
    (:Is%20Valid
      (bind _kingposition (Default|GetKingPosition _asbp_chess_game_mode (Variables|Default|GetTeam)))
      (LocalVariables|SetDirectionToKing (- _kingposition (Transformation|GetActorLocation)))
      (bind (_outhit _returnvalue_2) (Collision|LineTraceByChannel _returnvalue (+ _returnvalue (* (LocalVariables|GetDirectionToKing) -8e+02)) "TraceTypeQuery3" false 0 "None")) ; Pieces can only be pinned by the queen, rook, and bishop
      (if _returnvalue_2
        (if (>= (Math|Float|Absolute(Float) (.x (LocalVariables|GetDirectionToKing))) 1e+01) ; True means check diagonals
          (bind _asbp_bishop (Utilities|Casting|CastToBP_Bishop (.hitactor _outhit))
            (:then
              (Variables|Default|SetbIsPinned (Utilities|Enum|NotEqual(Enum) (Variables|Default|GetTeam) (Variables|BP_BaseChessPiece_C|GetTeam _asbp_bishop))))
            (:CastFailed
              (bind _asbp_queen (Utilities|Casting|CastToBP_Queen (.hitactor _outhit) :!label _label)
                (:then
                  (Variables|Default|SetbIsPinned (Utilities|Enum|NotEqual(Enum) (Variables|Default|GetTeam) (Variables|BP_BaseChessPiece_C|GetTeam _asbp_queen))))
                (:CastFailed
                  (Variables|Default|SetbIsPinned false :!label _label_2)))))
          (else
            (bind _asbp_rook (Utilities|Casting|CastToBP_Rook (.hitactor _outhit))
              (:then
                (Variables|Default|SetbIsPinned (Utilities|Enum|NotEqual(Enum) (Variables|Default|GetTeam) (Variables|BP_BaseChessPiece_C|GetTeam _asbp_rook))))
              (:CastFailed
                (goto _label)))))
        (else
          (goto _label_2)))
      (return (Variables|Default|GetbIsPinned)))))