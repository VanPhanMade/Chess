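; Pawn chess piece that shows its legal moves, moves and captures, including en passant.
; Forward, double-step and diagonal marker components are toggled by line traces for occupancy and enemy team.
; When its king is checked by a single piece, it tests only captures or blocks of that attacker, also used to report valid moves.
; Moving destroys captured pieces, flags en passant eligibility after a double step and plays a board-hit sound.
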(event EventMove
  (params (NewLocation :type Vector :default "0, 0, 0"))
  (bind _returnvalue (Transformation|GetActorLocation))
  (if (Utilities|Operators|EqualEqual (Transformation|GetWorldLocation (Variables|Default|GetForward2)) NewLocation 0.1)
    (Variables|Default|SetCanBeEnPassant true)
    (else
      (Variables|Default|SetCanBeEnPassant false)))
  (bind _output_get (Variables|Default|SetNewLocation NewLocation))
  (bind (_outhit _returnvalue_2) (Collision|LineTraceByChannel _output_get (+ _output_get (* (Math|Vector|VectorUp) 1e+02)) "TraceTypeQuery3" false 0 "None"))
  (if _returnvalue_2 ; Destroy pieces on take locations
    (Actor|DestroyActor (.hitactor _outhit))
    (else
      (bind (_outhit_2 _returnvalue_3) (Collision|LineTraceByChannel _returnvalue (+ _returnvalue (Math|Vector|MakeVector (.x (Variables|Default|GetNewLocation)) 0.0 0.0)) "TraceTypeQuery1" false 0 "None"))
      (if _returnvalue_3
        (bind _asbp_pawn (Utilities|Casting|CastToBP_Pawn (.HitActor (Collision|BreakHitResult _outhit_2)))
          (:then
            (if (Variables|BP_Pawn_C|GetCanBeEnPassant _asbp_pawn)
              (Actor|DestroyActor _asbp_pawn)))
          (:CastFailed
            _)))))
  (Transformation|SetActorLocation (Variables|Default|GetNewLocation) false false)
  (Variables|Default|SetMoved true)
  (Class|FMODBlueprintStatics|PlayEventatLocation "/Game/FMOD/Events/SFX/PieceHitBoard.PieceHitBoard" (Math|Transform|MakeTransform (Transformation|GetActorLocation) "0, 0, 0" "1.000000,1.000000,1.000000")))

(event EventDeSelect
  (Rendering|SetVisibility (Variables|Default|GetStart) false false)
  (Rendering|Material|SetOverlayMaterial (Variables|Default|GetChessPiece) "/Game/Art/Materials/M_OutlineClear.M_OutlineClear" :!class /Script/Engine.MeshComponent)
  (Collision|SetCollisionEnabled (Variables|Default|GetTakeRight) "NoCollision"))

(event EventShowValidMoves
  (bind _forward (Variables|Default|GetForward))
  (bind _forward2 (Variables|Default|GetForward2))
  (bind _forward_2 (Variables|Default|GetForward))
  (bind _returnvalue (Transformation|GetWorldLocation _forward_2))
  (bind _returnvalue_2 (Transformation|GetWorldLocation _forward2))
  (bind _pieceking (Variables|Default|GetPieceKing)
    (:then
      (if (Variables|/Game/Blueprints/Actors/BP_King.BP_King_C|GetChecked _pieceking)
        (if (not (>= (Utilities|Array|Length (Variables|/Game/Blueprints/Actors/BP_King.BP_King_C|GetPiecesCheckingKing _pieceking)) 2))
          (Utilities|CanTakePiece (Variables|Default|GetTakeRight) (Utilities|Array|Get(acopy) (Variables|/Game/Blueprints/Actors/BP_King.BP_King_C|GetPiecesCheckingKing _pieceking)) ; First see if it can be taken
            (:Blocks
              _)
            (:NoBlock
              _))
          (Utilities|CanTakePiece (Variables|Default|GetTakeRight) (Utilities|Array|Get(acopy) (Variables|/Game/Blueprints/Actors/BP_King.BP_King_C|GetPiecesCheckingKing _pieceking))
            (:Blocks
              _)
            (:NoBlock
              _))
          (Utilities|CheckMoveCanBlockAttack (Utilities|Array|Get(acopy) (Variables|/Game/Blueprints/Actors/BP_King.BP_King_C|GetPiecesCheckingKing _pieceking)) _forward_2
            (:CanBlock
              (bind _returnvalue_3 (Collision|LineTraceByChannel _returnvalue (+ _returnvalue (Math|Vector|VectorUp)) "TraceTypeQuery3" false 0 "None"))
              (if _returnvalue_3
                (Rendering|SetVisibility _forward false false)
                (Collision|SetCollisionEnabled _forward "NoCollision")))
            (:CannotBeBlocked
              (if (not (Variables|Default|GetMoved))
                (Utilities|CheckMoveCanBlockAttack (Utilities|Array|Get(acopy) (Variables|/Game/Blueprints/Actors/BP_King.BP_King_C|GetPiecesCheckingKing _pieceking)) _forward2
                  (:CanBlock
                    (bind _returnvalue_4 (Collision|LineTraceByChannel _returnvalue_2 (+ _returnvalue_2 (Math|Vector|VectorUp)) "TraceTypeQuery3" false 0 "None"))
                    (if _returnvalue_4
                      (Rendering|SetVisibility _forward2 false false)
                      (Collision|SetCollisionEnabled _forward2 "NoCollision"))))))))
        (else
          (Utilities|CanTakePiece (Variables|Default|GetTakeRight)
            (:Blocks
              _)
            (:NoBlock
              _))
          (Utilities|CanTakePiece (Variables|Default|GetTakeLeft)
            (:Blocks
              _)
            (:NoBlock
              _))
          (Utilities|CanMoveForward (Variables|Default|GetForward))
          (if (not (Variables|Default|GetMoved))
            (Utilities|CanMoveForward (Variables|Default|GetForward2))))))
    (:else)))

(fn ConstructionScript
  (|CallParentFunction))

(fn ReturnNumberOfValidMoves
  (bind _forward (Variables|Default|GetForward))
  (bind _forward2 (Variables|Default|GetForward2))
  (bind _forward_2 (Variables|Default|GetForward))
  (bind _returnvalue (Transformation|GetWorldLocation _forward_2))
  (bind _returnvalue_2 (Transformation|GetWorldLocation _forward2))
  (bind _pieceking (Variables|Default|GetPieceKing)
    (:then
      (if (not (>= (Utilities|Array|Length (Variables|/Game/Blueprints/Actors/BP_King.BP_King_C|GetPiecesCheckingKing _pieceking)) 2))
        (Utilities|CanTakePiece (Variables|Default|GetTakeRight) (Utilities|Array|Get(acopy) (Variables|/Game/Blueprints/Actors/BP_King.BP_King_C|GetPiecesCheckingKing _pieceking)) ; First see if it can be taken
          (:Blocks
            (LocalVariables|SetNumberOfBlocks 1.0 :!label _label)
            (CallFunction|DeSelect :!label _label_2)
            (return (LocalVariables|GetNumberOfBlocks)))
          (:NoBlock
            (Utilities|CanTakePiece (Variables|Default|GetTakeRight) (Utilities|Array|Get(acopy) (Variables|/Game/Blueprints/Actors/BP_King.BP_King_C|GetPiecesCheckingKing _pieceking))
              (:Blocks
                (goto _label))
              (:NoBlock
                (Utilities|CheckMoveCanBlockAttack (Utilities|Array|Get(acopy) (Variables|/Game/Blueprints/Actors/BP_King.BP_King_C|GetPiecesCheckingKing _pieceking)) _forward_2
                  (:CanBlock
                    (bind _returnvalue_3 (Collision|LineTraceByChannel _returnvalue (+ _returnvalue (Math|Vector|VectorUp)) "TraceTypeQuery3" false 0 "None"))
                    (if _returnvalue_3
                      (Rendering|SetVisibility _forward false false)
                      (Collision|SetCollisionEnabled _forward "NoCollision")
                      (goto _label)
                      (else
                        (goto _label_2))))
                  (:CannotBeBlocked
                    (if (not (Variables|Default|GetMoved))
                      (Utilities|CheckMoveCanBlockAttack (Utilities|Array|Get(acopy) (Variables|/Game/Blueprints/Actors/BP_King.BP_King_C|GetPiecesCheckingKing _pieceking)) _forward2
                        (:CanBlock
                          (bind _returnvalue_4 (Collision|LineTraceByChannel _returnvalue_2 (+ _returnvalue_2 (Math|Vector|VectorUp)) "TraceTypeQuery3" false 0 "None"))
                          (if _returnvalue_4
                            (Rendering|SetVisibility _forward2 false false)
                            (Collision|SetCollisionEnabled _forward2 "NoCollision")
                            (goto _label)))))))))))))
    (:else
      (return (LocalVariables|GetNumberOfBlocks)))))