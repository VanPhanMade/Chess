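; Queen chess piece that shows its legal move squares when asked and hides them on deselect.
; BeginPlay groups pre-placed square components into eight directional arrays, walked outward until blocked, with line traces detecting board, pieces and obstructions.
; When its king is checked by one piece, only moves passing CheckMoveCanBlockAttack are sought.
; ReturnNumberOfValidMoves runs that same check search, stopping at the first success to report 1.
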(event EventBeginPlay
  (bind _forwards (Variables|Default|GetForwards))
  (bind _forwardlefts (Variables|Default|GetForwardLefts))
  (bind _lefts (Variables|Default|GetLefts))
  (bind _rights (Variables|Default|GetRights))
  (bind _backwards (Variables|Default|GetBackwards))
  (bind _backlefts (Variables|Default|GetBackLefts))
  (bind _backrights (Variables|Default|GetBackRights))
  (bind _forwardrights (Variables|Default|GetForwardRights))
  (|CallParentFunction)
  (Utilities|Array|Add _forwards (Variables|Components|GetForward1))
  (Utilities|Array|Add _forwards (Variables|Components|GetForward2))
  (Utilities|Array|Add _forwards (Variables|Components|GetForward3))
  (Utilities|Array|Add _forwards (Variables|Components|GetForward4))
  (Utilities|Array|Add _forwards (Variables|Components|GetForward5))
  (Utilities|Array|Add _forwards (Variables|Components|GetForward6))
  (Utilities|Array|Add _forwards (Variables|Components|GetForward7))
  (Utilities|Array|Add _forwardrights (Variables|Components|GetForwardRight))
  (Utilities|Array|Add _forwardrights (Variables|Components|GetForwardRight1))
  (Utilities|Array|Add _forwardrights (Variables|Components|GetForwardRight2))
  (Utilities|Array|Add _forwardrights (Variables|Components|GetForwardRight3))
  (Utilities|Array|Add _forwardrights (Variables|Components|GetForwardRight4))
  (Utilities|Array|Add _forwardrights (Variables|Components|GetForwardRight5))
  (Utilities|Array|Add _forwardrights (Variables|Components|GetForwardRight6))
  (Utilities|Array|Add _forwardlefts (Variables|Components|GetForwardLeft))
  (Utilities|Array|Add _forwardlefts (Variables|Components|GetForwardLeft1))
  (Utilities|Array|Add _forwardlefts (Variables|Components|GetForwardLeft2))
  (Utilities|Array|Add _forwardlefts (Variables|Components|GetForwardLeft3))
  (Utilities|Array|Add _forwardlefts (Variables|Components|GetForwardLeft4))
  (Utilities|Array|Add _forwardlefts (Variables|Components|GetForwardLeft5))
  (Utilities|Array|Add _forwardlefts (Variables|Components|GetForwardLeft6))
  (Utilities|Array|Add _lefts (Variables|Components|GetLeft1))
  (Utilities|Array|Add _lefts (Variables|Components|GetLeft2))
  (Utilities|Array|Add _lefts (Variables|Components|GetLeft3))
  (Utilities|Array|Add _lefts (Variables|Components|GetLeft4))
  (Utilities|Array|Add _lefts (Variables|Components|GetLeft5))
  (Utilities|Array|Add _lefts (Variables|Components|GetLeft6))
  (Utilities|Array|Add _lefts (Variables|Components|GetLeft7))
  (Utilities|Array|Add _rights (Variables|Components|GetRight1))
  (Utilities|Array|Add _rights (Variables|Components|GetRight2))
  (Utilities|Array|Add _rights (Variables|Components|GetRight3))
  (Utilities|Array|Add _rights (Variables|Components|GetRight4))
  (Utilities|Array|Add _rights (Variables|Components|GetRight5))
  (Utilities|Array|Add _rights (Variables|Components|GetRight6))
  (Utilities|Array|Add _rights (Variables|Components|GetRight7))
  (Utilities|Array|Add _backwards (Variables|Components|GetBack1))
  (Utilities|Array|Add _backwards (Variables|Components|GetBack2))
  (Utilities|Array|Add _backwards (Variables|Components|GetBack3))
  (Utilities|Array|Add _backwards (Variables|Components|GetBack4))
  (Utilities|Array|Add _backwards (Variables|Components|GetBack5))
  (Utilities|Array|Add _backwards (Variables|Components|GetBack6))
  (Utilities|Array|Add _backwards (Variables|Components|GetBack7))
  (Utilities|Array|Add _backlefts (Variables|Components|GetBackLeft))
  (Utilities|Array|Add _backlefts (Variables|Components|GetBackLeft1))
  (Utilities|Array|Add _backlefts (Variables|Components|GetBackLeft2))
  (Utilities|Array|Add _backlefts (Variables|Components|GetBackLeft3))
  (Utilities|Array|Add _backlefts (Variables|Components|GetBackLeft4))
  (Utilities|Array|Add _backlefts (Variables|Components|GetBackLeft5))
  (Utilities|Array|Add _backlefts (Variables|Components|GetBackLeft6))
  (Utilities|Array|Add _backrights (Variables|Components|GetBackRight))
  (Utilities|Array|Add _backrights (Variables|Components|GetBackRight1))
  (Utilities|Array|Add _backrights (Variables|Components|GetBackRight2))
  (Utilities|Array|Add _backrights (Variables|Components|GetBackRight3))
  (Utilities|Array|Add _backrights (Variables|Components|GetBackRight4))
  (Utilities|Array|Add _backrights (Variables|Components|GetBackRight5))
  (Utilities|Array|Add _backrights (Variables|Components|GetBackRight6)))

(event EventDeSelect
  (Rendering|Material|SetOverlayMaterial (Variables|Default|GetChessPiece) "/Game/Art/Materials/M_OutlineClear.M_OutlineClear" :!class /Script/Engine.MeshComponent)
  (for _array_element (Variables|Default|GetForwards)
    (Collision|SetCollisionEnabled _array_element "NoCollision")
    (Rendering|SetVisibility _array_element false false))
  (for _array_element_2 (Variables|Default|GetForwardRights)
    (Collision|SetCollisionEnabled _array_element_2 "NoCollision")
    (Rendering|SetVisibility _array_element_2 false false))
  (for _array_element_3 (Variables|Default|GetForwardLefts)
    (Collision|SetCollisionEnabled _array_element_3 "NoCollision")
    (Rendering|SetVisibility _array_element_3 false false))
  (for _array_element_4 (Variables|Default|GetLefts)
    (Collision|SetCollisionEnabled _array_element_4 "NoCollision")
    (Rendering|SetVisibility _array_element_4 false false))
  (for _array_element_5 (Variables|Default|GetRights)
    (Collision|SetCollisionEnabled _array_element_5 "NoCollision")
    (Rendering|SetVisibility _array_element_5 false false))
  (for _array_element_6 (Variables|Default|GetBackwards)
    (Collision|SetCollisionEnabled _array_element_6 "NoCollision")
    (Rendering|SetVisibility _array_element_6 false false))
  (for _array_element_7 (Variables|Default|GetBackLefts)
    (Collision|SetCollisionEnabled _array_element_7 "NoCollision")
    (Rendering|SetVisibility _array_element_7 false false))
  (for _array_element_8 (Variables|Default|GetBackRights)
    (Collision|SetCollisionEnabled _array_element_8 "NoCollision")
    (Rendering|SetVisibility _array_element_8 false false)))

(event EventShowValidMoves
  (bind _pieceking (Variables|Default|GetPieceKing)
    (:then
      (if (Variables|/Game/Blueprints/Actors/BP_King.BP_King_C|GetChecked _pieceking)
        (if (< (Utilities|Array|Length (Variables|/Game/Blueprints/Actors/BP_King.BP_King_C|GetPiecesCheckingKing _pieceking)) 2)
          (bind _array_element (Utilities|Array|ForEachLoopwithBreak (Variables|Default|GetForwards) :!label _label)
            (:LoopBody
              (Utilities|CalculateifPieceinPath _array_element (Utilities|Array|Get(acopy) (Variables|/Game/Blueprints/Actors/BP_King.BP_King_C|GetPiecesCheckingKing _pieceking))
                (:SpotClear
                  _)
                (:PieceInTheWay
                  (goto _label Break))
                (:EnemyToTakeFound
                  _))
              (Utilities|CheckMoveCanBlockAttack (Utilities|Array|Get(acopy) (Variables|/Game/Blueprints/Actors/BP_King.BP_King_C|GetPiecesCheckingKing _pieceking)) _array_element
                (:CanBlock
                  (goto _label Break))))
            (:Completed
              (bind _array_element_2 (Utilities|Array|ForEachLoopwithBreak (Variables|Default|GetForwardRights) :!label _label_2)
                (:LoopBody
                  (Utilities|CalculateifPieceinPath _array_element_2 (Utilities|Array|Get(acopy) (Variables|/Game/Blueprints/Actors/BP_King.BP_King_C|GetPiecesCheckingKing _pieceking))
                    (:SpotClear
                      _)
                    (:PieceInTheWay
                      (goto _label_2 Break))
                    (:EnemyToTakeFound
                      _))
                  (Utilities|CheckMoveCanBlockAttack (Utilities|Array|Get(acopy) (Variables|/Game/Blueprints/Actors/BP_King.BP_King_C|GetPiecesCheckingKing _pieceking)) _array_element_2
                    (:CanBlock
                      (goto _label_2 Break))))
                (:Completed
                  (bind _array_element_3 (Utilities|Array|ForEachLoopwithBreak (Variables|Default|GetForwardLefts) :!label _label_3)
                    (:LoopBody
                      (Utilities|CalculateifPieceinPath _array_element_3 (Utilities|Array|Get(acopy) (Variables|/Game/Blueprints/Actors/BP_King.BP_King_C|GetPiecesCheckingKing _pieceking))
                        (:SpotClear
                          _)
                        (:PieceInTheWay
                          (goto _label_3 Break))
                        (:EnemyToTakeFound
                          _))
                      (Utilities|CheckMoveCanBlockAttack (Utilities|Array|Get(acopy) (Variables|/Game/Blueprints/Actors/BP_King.BP_King_C|GetPiecesCheckingKing _pieceking)) _array_element_3
                        (:CanBlock
                          (goto _label_3 Break))))
                    (:Completed
                      (bind _array_element_4 (Utilities|Array|ForEachLoopwithBreak (Variables|Default|GetLefts) :!label _label_4)
                        (:LoopBody
                          (Utilities|CalculateifPieceinPath _array_element_4 (Utilities|Array|Get(acopy) (Variables|/Game/Blueprints/Actors/BP_King.BP_King_C|GetPiecesCheckingKing _pieceking))
                            (:SpotClear
                              _)
                            (:PieceInTheWay
                              (goto _label_4 Break))
                            (:EnemyToTakeFound
                              _))
                          (Utilities|CheckMoveCanBlockAttack (Utilities|Array|Get(acopy) (Variables|/Game/Blueprints/Actors/BP_King.BP_King_C|GetPiecesCheckingKing _pieceking)) _array_element_4
                            (:CanBlock
                              (goto _label_4 Break))))
                        (:Completed
                          (bind _array_element_5 (Utilities|Array|ForEachLoopwithBreak (Variables|Default|GetRights) :!label _label_5)
                            (:LoopBody
                              (Utilities|CalculateifPieceinPath _array_element_5 (Utilities|Array|Get(acopy) (Variables|/Game/Blueprints/Actors/BP_King.BP_King_C|GetPiecesCheckingKing _pieceking))
                                (:SpotClear
                                  _)
                                (:PieceInTheWay
                                  (goto _label_5 Break))
                                (:EnemyToTakeFound
                                  _))
                              (Utilities|CheckMoveCanBlockAttack (Utilities|Array|Get(acopy) (Variables|/Game/Blueprints/Actors/BP_King.BP_King_C|GetPiecesCheckingKing _pieceking)) _array_element_5
                                (:CanBlock
                                  (goto _label_5 Break))))
                            (:Completed
                              (bind _array_element_6 (Utilities|Array|ForEachLoopwithBreak (Variables|Default|GetBackwards) :!label _label_6)
                                (:LoopBody
                                  (Utilities|CalculateifPieceinPath _array_element_6 (Utilities|Array|Get(acopy) (Variables|/Game/Blueprints/Actors/BP_King.BP_King_C|GetPiecesCheckingKing _pieceking))
                                    (:SpotClear
                                      _)
                                    (:PieceInTheWay
                                      (goto _label_6 Break))
                                    (:EnemyToTakeFound
                                      _))
                                  (Utilities|CheckMoveCanBlockAttack (Utilities|Array|Get(acopy) (Variables|/Game/Blueprints/Actors/BP_King.BP_King_C|GetPiecesCheckingKing _pieceking)) _array_element_6
                                    (:CanBlock
                                      (goto _label_6 Break))))
                                (:Completed
                                  (bind _array_element_7 (Utilities|Array|ForEachLoopwithBreak (Variables|Default|GetBackLefts) :!label _label_7)
                                    (:LoopBody
                                      (Utilities|CalculateifPieceinPath _array_element_7 (Utilities|Array|Get(acopy) (Variables|/Game/Blueprints/Actors/BP_King.BP_King_C|GetPiecesCheckingKing _pieceking))
                                        (:SpotClear
                                          _)
                                        (:PieceInTheWay
                                          (goto _label_7 Break))
                                        (:EnemyToTakeFound
                                          _))
                                      (Utilities|CheckMoveCanBlockAttack (Utilities|Array|Get(acopy) (Variables|/Game/Blueprints/Actors/BP_King.BP_King_C|GetPiecesCheckingKing _pieceking)) _array_element_7
                                        (:CanBlock
                                          (goto _label_7 Break))))
                                    (:Completed
                                      (bind _array_element_8 (Utilities|Array|ForEachLoopwithBreak (Variables|Default|GetBackRights) :!label _label_8)
                                        (:LoopBody
                                          (Utilities|CalculateifPieceinPath _array_element_8 (Utilities|Array|Get(acopy) (Variables|/Game/Blueprints/Actors/BP_King.BP_King_C|GetPiecesCheckingKing _pieceking))
                                            (:SpotClear
                                              _)
                                            (:PieceInTheWay
                                              (goto _label_8 Break))
                                            (:EnemyToTakeFound
                                              _))
                                          (Utilities|CheckMoveCanBlockAttack (Utilities|Array|Get(acopy) (Variables|/Game/Blueprints/Actors/BP_King.BP_King_C|GetPiecesCheckingKing _pieceking)) _array_element_8
                                            (:CanBlock
                                              (goto _label_8 Break))))))))))))))))))))
        (else
          (bind _array_element_9 (Utilities|Array|ForEachLoopwithBreak (Variables|Default|GetForwards) :!label _label_9)
            (:LoopBody
              (Utilities|CalculateValidMove _array_element_9
                (:InValidMove
                  (goto _label_9 Break))
                (:PieceToTake
                  (goto _label_9 Break))))
            (:Completed
              (bind _array_element_10 (Utilities|Array|ForEachLoopwithBreak (Variables|Default|GetForwardRights) :!label _label_10)
                (:LoopBody
                  (Utilities|CalculateValidMove _array_element_10
                    (:InValidMove
                      (goto _label_10 Break))
                    (:PieceToTake
                      (goto _label_10 Break))))
                (:Completed
                  (bind _array_element_11 (Utilities|Array|ForEachLoopwithBreak (Variables|Default|GetForwardLefts) :!label _label_11)
                    (:LoopBody
                      (Utilities|CalculateValidMove _array_element_11
                        (:InValidMove
                          (goto _label_11 Break))
                        (:PieceToTake
                          (goto _label_11 Break))))
                    (:Completed
                      (bind _array_element_12 (Utilities|Array|ForEachLoopwithBreak (Variables|Default|GetLefts) :!label _label_12)
                        (:LoopBody
                          (Utilities|CalculateValidMove _array_element_12
                            (:InValidMove
                              (goto _label_12 Break))
                            (:PieceToTake
                              (goto _label_12 Break))))
                        (:Completed
                          (bind _array_element_13 (Utilities|Array|ForEachLoopwithBreak (Variables|Default|GetRights) :!label _label_13)
                            (:LoopBody
                              (Utilities|CalculateValidMove _array_element_13
                                (:InValidMove
                                  (goto _label_13 Break))
                                (:PieceToTake
                                  (goto _label_13 Break))))
                            (:Completed
                              (bind _array_element_14 (Utilities|Array|ForEachLoopwithBreak (Variables|Default|GetBackwards) :!label _label_14)
                                (:LoopBody
                                  (Utilities|CalculateValidMove _array_element_14
                                    (:InValidMove
                                      (goto _label_14 Break))
                                    (:PieceToTake
                                      (goto _label_14 Break))))
                                (:Completed
                                  (bind _array_element_15 (Utilities|Array|ForEachLoopwithBreak (Variables|Default|GetBackLefts) :!label _label_15)
                                    (:LoopBody
                                      (Utilities|CalculateValidMove _array_element_15
                                        (:InValidMove
                                          (goto _label_15 Break))
                                        (:PieceToTake
                                          (goto _label_15 Break))))
                                    (:Completed
                                      (bind _array_element_16 (Utilities|Array|ForEachLoopwithBreak (Variables|Default|GetBackRights) :!label _label_16)
                                        (:LoopBody
                                          (Utilities|CalculateValidMove _array_element_16
                                            (:InValidMove
                                              (goto _label_16 Break))
                                            (:PieceToTake
                                              (goto _label_16 Break))))))))))))))))))))))
    (:else)))

(fn ConstructionScript
  (|CallParentFunction))

(fn ReturnNumberOfValidMoves
  (bind _pieceking (Variables|Default|GetPieceKing)
    (:then
      (if (< (Utilities|Array|Length (Variables|/Game/Blueprints/Actors/BP_King.BP_King_C|GetPiecesCheckingKing _pieceking)) 2)
        (bind _array_element (Utilities|Array|ForEachLoopwithBreak (Variables|Default|GetForwards) :!label _label)
          (:LoopBody
            (Utilities|CalculateifPieceinPath _array_element (Utilities|Array|Get(acopy) (Variables|/Game/Blueprints/Actors/BP_King.BP_King_C|GetPiecesCheckingKing _pieceking))
              (:SpotClear
                _)
              (:PieceInTheWay
                (goto _label Break))
              (:EnemyToTakeFound
                _))
            (Utilities|CheckMoveCanBlockAttack (Utilities|Array|Get(acopy) (Variables|/Game/Blueprints/Actors/BP_King.BP_King_C|GetPiecesCheckingKing _pieceking)) _array_element
              (:CanBlock
                (LocalVariables|SetValidMoves 1.0 :!label _label_2))))
          (:Completed
            (bind _array_element_2 (Utilities|Array|ForEachLoopwithBreak (Variables|Default|GetForwardRights) :!label _label_3)
              (:LoopBody
                (Utilities|CalculateifPieceinPath _array_element_2 (Utilities|Array|Get(acopy) (Variables|/Game/Blueprints/Actors/BP_King.BP_King_C|GetPiecesCheckingKing _pieceking))
                  (:SpotClear
                    _)
                  (:PieceInTheWay
                    (goto _label_3 Break))
                  (:EnemyToTakeFound
                    _))
                (Utilities|CheckMoveCanBlockAttack (Utilities|Array|Get(acopy) (Variables|/Game/Blueprints/Actors/BP_King.BP_King_C|GetPiecesCheckingKing _pieceking)) _array_element_2
                  (:CanBlock
                    (goto _label_2))))
              (:Completed
                (bind _array_element_3 (Utilities|Array|ForEachLoopwithBreak (Variables|Default|GetForwardLefts) :!label _label_4)
                  (:LoopBody
                    (Utilities|CalculateifPieceinPath _array_element_3 (Utilities|Array|Get(acopy) (Variables|/Game/Blueprints/Actors/BP_King.BP_King_C|GetPiecesCheckingKing _pieceking))
                      (:SpotClear
                        _)
                      (:PieceInTheWay
                        (goto _label_4 Break))
                      (:EnemyToTakeFound
                        _))
                    (Utilities|CheckMoveCanBlockAttack (Utilities|Array|Get(acopy) (Variables|/Game/Blueprints/Actors/BP_King.BP_King_C|GetPiecesCheckingKing _pieceking)) _array_element_3
                      (:CanBlock
                        (goto _label_2))))
                  (:Completed
                    (bind _array_element_4 (Utilities|Array|ForEachLoopwithBreak (Variables|Default|GetLefts) :!label _label_5)
                      (:LoopBody
                        (Utilities|CalculateifPieceinPath _array_element_4 (Utilities|Array|Get(acopy) (Variables|/Game/Blueprints/Actors/BP_King.BP_King_C|GetPiecesCheckingKing _pieceking))
                          (:SpotClear
                            _)
                          (:PieceInTheWay
                            (goto _label_5 Break))
                          (:EnemyToTakeFound
                            _))
                        (Utilities|CheckMoveCanBlockAttack (Utilities|Array|Get(acopy) (Variables|/Game/Blueprints/Actors/BP_King.BP_King_C|GetPiecesCheckingKing _pieceking)) _array_element_4
                          (:CanBlock
                            (goto _label_2))))
                      (:Completed
                        (bind _array_element_5 (Utilities|Array|ForEachLoopwithBreak (Variables|Default|GetRights) :!label _label_6)
                          (:LoopBody
                            (Utilities|CalculateifPieceinPath _array_element_5 (Utilities|Array|Get(acopy) (Variables|/Game/Blueprints/Actors/BP_King.BP_King_C|GetPiecesCheckingKing _pieceking))
                              (:SpotClear
                                _)
                              (:PieceInTheWay
                                (goto _label_6 Break))
                              (:EnemyToTakeFound
                                _))
                            (Utilities|CheckMoveCanBlockAttack (Utilities|Array|Get(acopy) (Variables|/Game/Blueprints/Actors/BP_King.BP_King_C|GetPiecesCheckingKing _pieceking)) _array_element_5
                              (:CanBlock
                                (goto _label_2))))
                          (:Completed
                            (bind _array_element_6 (Utilities|Array|ForEachLoopwithBreak (Variables|Default|GetBackwards) :!label _label_7)
                              (:LoopBody
                                (Utilities|CalculateifPieceinPath _array_element_6 (Utilities|Array|Get(acopy) (Variables|/Game/Blueprints/Actors/BP_King.BP_King_C|GetPiecesCheckingKing _pieceking))
                                  (:SpotClear
                                    _)
                                  (:PieceInTheWay
                                    (goto _label_7 Break))
                                  (:EnemyToTakeFound
                                    _))
                                (Utilities|CheckMoveCanBlockAttack (Utilities|Array|Get(acopy) (Variables|/Game/Blueprints/Actors/BP_King.BP_King_C|GetPiecesCheckingKing _pieceking)) _array_element_6
                                  (:CanBlock
                                    (goto _label_2))))
                              (:Completed
                                (bind _array_element_7 (Utilities|Array|ForEachLoopwithBreak (Variables|Default|GetBackLefts) :!label _label_8)
                                  (:LoopBody
                                    (Utilities|CalculateifPieceinPath _array_element_7 (Utilities|Array|Get(acopy) (Variables|/Game/Blueprints/Actors/BP_King.BP_King_C|GetPiecesCheckingKing _pieceking))
                                      (:SpotClear
                                        _)
                                      (:PieceInTheWay
                                        (goto _label_8 Break))
                                      (:EnemyToTakeFound
                                        _))
                                    (Utilities|CheckMoveCanBlockAttack (Utilities|Array|Get(acopy) (Variables|/Game/Blueprints/Actors/BP_King.BP_King_C|GetPiecesCheckingKing _pieceking)) _array_element_7
                                      (:CanBlock
                                        (goto _label_2))))
                                  (:Completed
                                    (bind _array_element_8 (Utilities|Array|ForEachLoopwithBreak (Variables|Default|GetBackRights) :!label _label_9)
                                      (:LoopBody
                                        (Utilities|CalculateifPieceinPath _array_element_8 (Utilities|Array|Get(acopy) (Variables|/Game/Blueprints/Actors/BP_King.BP_King_C|GetPiecesCheckingKing _pieceking))
                                          (:SpotClear
                                            _)
                                          (:PieceInTheWay
                                            (goto _label_9 Break))
                                          (:EnemyToTakeFound
                                            _))
                                        (Utilities|CheckMoveCanBlockAttack (Utilities|Array|Get(acopy) (Variables|/Game/Blueprints/Actors/BP_King.BP_King_C|GetPiecesCheckingKing _pieceking)) _array_element_8
                                          (:CanBlock
                                            (goto _label_2))))
                                      (:Completed
                                        _))))))))))))))))
        (CallFunction|DeSelect)
        (return (LocalVariables|GetValidMoves))))
    (:else
      (return (LocalVariables|GetValidMoves)))))