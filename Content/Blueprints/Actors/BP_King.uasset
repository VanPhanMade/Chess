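; King chess piece that registers with BP_ChessGameMode and shows or hides its move-square components on selection.
; Unless checked, it validates squares by tracing for board and occupants, omitting Left; castling is an empty stub.
; Check detection traces eight lines and eight knight offsets derived from square components.
; It records any enemy piece hit, regardless of type, and sets Checked; CardinalDirections is never cleared between runs.
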(event EventDeSelect
  (bind _castleleft (Variables|Default|GetCastleLeft))
  (Rendering|Material|SetOverlayMaterial (Variables|Default|GetChessPiece) "/Game/Art/Materials/M_OutlineClear.M_OutlineClear" :!class /Script/Engine.MeshComponent)
  (Collision|SetCollisionEnabled _castleleft "NoCollision")
  (Rendering|SetVisibility _castleleft false false))

(event EventShowValidMoves
  (if (not (Variables|Default|GetChecked))
    (Utilities|CalculateValidMove (Variables|Default|GetBackLeft)
      (:ValidMove
        _)
      (:InValidMove
        _)
      (:PieceToTake
        _))
    (Utilities|CalculateValidMove (Variables|Default|GetBackRight)
      (:ValidMove
        _)
      (:InValidMove
        _)
      (:PieceToTake
        _))
    (Utilities|CalculateValidMove (Variables|Default|GetBack)
      (:ValidMove
        _)
      (:InValidMove
        _)
      (:PieceToTake
        _))
    (Utilities|CalculateValidMove (Variables|Default|GetRight)
      (:ValidMove
        _)
      (:InValidMove
        _)
      (:PieceToTake
        _))
    (Utilities|CalculateValidMove (Variables|Default|GetForwardLeft)
      (:ValidMove
        _)
      (:InValidMove
        _)
      (:PieceToTake
        _))
    (Utilities|CalculateValidMove (Variables|Default|GetForwardRight)
      (:ValidMove
        _)
      (:InValidMove
        _)
      (:PieceToTake
        _))
    (Utilities|CalculateValidMove (Variables|Default|GetForward)
      (:ValidMove
        _)
      (:InValidMove
        _)
      (:PieceToTake
        _))
    (if (not (Variables|Default|GetMoved))
      (Utilities|CalculateCastles (Variables|Default|GetCastleLeft)
        (:Out
          (Utilities|CalculateCastles (Variables|Default|GetCastleRight)))))))

(event EventBeginPlay
  (bind _asbp_chess_game_mode (Utilities|Casting|CastToBP_ChessGameMode (Game|GetGameMode)))
  (Utilities|IsValid _asbp_chess_game_mode
    (:Is%20Valid
      (Default|AddKings _asbp_chess_game_mode self))))

(fn ConstructionScript
  (|CallParentFunction))

(fn CalculateinCheck
  (bind _returnvalue (Transformation|GetActorLocation))
  (bind _cardinaldirections (LocalVariables|GetCardinalDirections))
  (bind _piecescheckingking (Variables|Default|GetPiecesCheckingKing))
  (bind _knightpositions (LocalVariables|GetKnightPositions))
  (bind _returnvalue_2 (Utilities|Array|Length _piecescheckingking))
  (bind _output_get (LocalVariables|SetForwardDirection (- (Transformation|GetWorldLocation (Variables|Default|GetForward)) (Transformation|GetActorLocation))))
  (LocalVariables|SetBackDirection (* _output_get -1.0))
  (bind _output_get_2 (LocalVariables|SetRightDirection (- (Transformation|GetWorldLocation (Variables|Default|GetRight)) (Transformation|GetActorLocation))))
  (LocalVariables|SetLeftDirection (* _output_get_2 -1.0))
  (bind _output_get_3 (LocalVariables|SetForwardRightDirection (- (Transformation|GetWorldLocation (Variables|Default|GetForwardRight)) (Transformation|GetActorLocation))))
  (LocalVariables|SetBackLeftDirection (* _output_get_3 -1.0))
  (bind _output_get_4 (LocalVariables|SetForwardLeftDirection (- (Transformation|GetWorldLocation (Variables|Default|GetForwardLeft)) (Transformation|GetActorLocation))))
  (LocalVariables|SetBackRightDirection (* _output_get_4 -1.0))
  (LocalVariables|SetKnightForwardLeftDirection (+ (* (LocalVariables|GetForwardDirection) 2.0) (LocalVariables|GetLeftDirection)))
  (LocalVariables|SetKnightForwardRightDirection (+ (* (LocalVariables|GetForwardDirection) 2.0) (LocalVariables|GetRightDirection)))
  (LocalVariables|SetKnightRightForwardDirection (+ (LocalVariables|GetForwardDirection) (* (LocalVariables|GetRightDirection) 2.0)))
  (LocalVariables|SetKnightLeftForwardDirection (+ (LocalVariables|GetForwardDirection) (* (LocalVariables|GetLeftDirection) 2.0)))
  (LocalVariables|SetKnightRightBackDirection (+ (LocalVariables|GetBackDirection) (* (LocalVariables|GetRightDirection) 2.0)))
  (LocalVariables|SetKnightLeftBackDirection (+ (LocalVariables|GetBackDirection) (* (LocalVariables|GetLeftDirection) 2.0)))
  (LocalVariables|SetKnightBackLeftDirection (+ (LocalVariables|GetLeftDirection) (* (LocalVariables|GetBackDirection) 2.0)))
  (LocalVariables|SetKnightBackRightDirection (+ (LocalVariables|GetRightDirection) (* (LocalVariables|GetBackDirection) 2.0)))
  (Utilities|Array|Clear _knightpositions)
  (Utilities|Array|Add _knightpositions (LocalVariables|GetKnightForwardLeftDirection))
  (Utilities|Array|Add _knightpositions (LocalVariables|GetKnightForwardRightDirection))
  (Utilities|Array|Add _knightpositions (LocalVariables|GetKnightRightForwardDirection))
  (Utilities|Array|Add _knightpositions (LocalVariables|GetKnightLeftForwardDirection))
  (Utilities|Array|Add _knightpositions (LocalVariables|GetKnightRightBackDirection))
  (Utilities|Array|Add _knightpositions (LocalVariables|GetKnightLeftBackDirection))
  (Utilities|Array|Add _knightpositions (LocalVariables|GetKnightBackLeftDirection))
  (Utilities|Array|Add _knightpositions (LocalVariables|GetKnightBackRightDirection))
  (Utilities|Array|Clear (Variables|Default|GetPiecesCheckingKing))
  (Utilities|Array|Add _cardinaldirections (LocalVariables|GetForwardDirection))
  (Utilities|Array|Add _cardinaldirections (LocalVariables|GetBackDirection))
  (Utilities|Array|Add _cardinaldirections (LocalVariables|GetRightDirection))
  (Utilities|Array|Add _cardinaldirections (LocalVariables|GetLeftDirection))
  (Utilities|Array|Add _cardinaldirections (LocalVariables|GetForwardRightDirection))
  (Utilities|Array|Add _cardinaldirections (LocalVariables|GetBackLeftDirection))
  (Utilities|Array|Add _cardinaldirections (LocalVariables|GetForwardLeftDirection))
  (Utilities|Array|Add _cardinaldirections (LocalVariables|GetBackRightDirection))
  (for _array_element (LocalVariables|GetCardinalDirections)
    (Utilities|CalculateinCheck _returnvalue (+ _returnvalue (* _array_element 8.0))))
  (for _array_element_2 (LocalVariables|GetKnightPositions)
    (Utilities|CalculateinCheck (+ _array_element_2 (Transformation|GetActorLocation)) (+ (+ _array_element_2 (Transformation|GetActorLocation)) (* (Math|Vector|VectorUp) 1e+02))))
  (if (== _returnvalue_2 0)
    (bind _output_get_5 (LocalVariables|SetbIsInCheck false))
    (Variables|Default|SetChecked _output_get_5)
    (Development|PrintString "Not in check")
    (elif (>= _returnvalue_2 2)
      (bind _output_get_6 (LocalVariables|SetbIsInCheck true))
      (Variables|Default|SetChecked _output_get_6)
      (Development|PrintString "One piece check")
      (else
        (bind _output_get_7 (LocalVariables|SetbIsInCheck true))
        (Variables|Default|SetChecked _output_get_7)
        (Development|PrintString "One piece check"))))
  (return (LocalVariables|GetbIsInCheck)))