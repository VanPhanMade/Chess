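; Bishop chess piece that shows its legal diagonal moves by toggling pre-placed marker components, grouped at BeginPlay into four arrays of seven.
; Normally, each diagonal is walked using downward traces for board and occupant, revealing squares until blocked or an enemy is capturable.
; When its king has a single attacker, path and block helpers filter the moves instead.
; ReturnNumberOfValidMoves reuses that check, stopping at the first answer to the attack.
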(event EventShowValidMoves
  (bind _pieceking (Variables|Default|GetPieceKing)
    (:then
      (if (Variables|/Game/Blueprints/Actors/BP_King.BP_King_C|GetChecked _pieceking)
        (if (< (Utilities|Array|Length (Variables|/Game/Blueprints/Actors/BP_King.BP_King_C|GetPiecesCheckingKing _pieceking)) 2)
          (bind _array_element (Utilities|Array|ForEachLoopwithBreak (Variables|Default|GetBackLefts) :!label _label)
            (:LoopBody
              (Utilities|CalculateifPieceinPath _array_element (Utilities|Array|Get(acopy) (Variables|/Game/Blueprints/Actors/BP_King.BP_King_C|GetPiecesCheckingKing _pieceking))
                (:SpotClear
                  _)
                (:PieceInTheWay
                  (goto _label Break))
                (:EnemyToTakeFound
                  _))
              (Utilities|CheckMoveCanBlockAttack (Utilities|Array|Get(acopy) (Variables|/Game/Blueprints/Actors/BP_King.BP_King_C|GetPiecesCheckingKing _pieceking)) _array_element
                (:CanBlock
                  (goto _label Break))))
            (:Completed
              (bind _array_element_2 (Utilities|Array|ForEachLoopwithBreak (Variables|Default|GetBackRights) :!label _label_2)
                (:LoopBody
                  (Utilities|CalculateifPieceinPath _array_element_2 (Utilities|Array|Get(acopy) (Variables|/Game/Blueprints/Actors/BP_King.BP_King_C|GetPiecesCheckingKing _pieceking))
                    (:SpotClear
                      _)
                    (:PieceInTheWay
                      (goto _label_2 Break))
                    (:EnemyToTakeFound
                      _))
                  (Utilities|CheckMoveCanBlockAttack (Utilities|Array|Get(acopy) (Variables|/Game/Blueprints/Actors/BP_King.BP_King_C|GetPiecesCheckingKing _pieceking)) _array_element_2
                    (:CanBlock
                      (goto _label_2 Break))))
                (:Completed
                  (bind _array_element_3 (Utilities|Array|ForEachLoopwithBreak (Variables|Default|GetForwardLefts) :!label _label_3)
                    (:LoopBody
                      (Utilities|CalculateifPieceinPath _array_element_3 (Utilities|Array|Get(acopy) (Variables|/Game/Blueprints/Actors/BP_King.BP_King_C|GetPiecesCheckingKing _pieceking))
                        (:SpotClear
                          _)
                        (:PieceInTheWay
                          (goto _label_3 Break))
                        (:EnemyToTakeFound
                          _))
                      (Utilities|CheckMoveCanBlockAttack (Utilities|Array|Get(acopy) (Variables|/Game/Blueprints/Actors/BP_King.BP_King_C|GetPiecesCheckingKing _pieceking)) _array_element_3
                        (:CanBlock
                          (goto _label_3 Break))))
                    (:Completed
                      (bind _array_element_4 (Utilities|Array|ForEachLoopwithBreak (Variables|Default|GetForwardRights) :!label _label_4)
                        (:LoopBody
                          (Utilities|CalculateifPieceinPath _array_element_4 (Utilities|Array|Get(acopy) (Variables|/Game/Blueprints/Actors/BP_King.BP_King_C|GetPiecesCheckingKing _pieceking))
                            (:SpotClear
                              _)
                            (:PieceInTheWay
                              (goto _label_4 Break))
                            (:EnemyToTakeFound
                              _))
                          (Utilities|CheckMoveCanBlockAttack (Utilities|Array|Get(acopy) (Variables|/Game/Blueprints/Actors/BP_King.BP_King_C|GetPiecesCheckingKing _pieceking)) _array_element_4
                            (:CanBlock
                              (goto _label_4 Break))))))))))))
        (else
          (bind _array_element_5 (Utilities|Array|ForEachLoopwithBreak (Variables|Default|GetBackLefts) :!label _label_5)
            (:LoopBody
              (Utilities|CalculateValidMove _array_element_5
                (:InValidMove
                  (goto _label_5 Break))
                (:PieceToTake
                  (goto _label_5 Break))))
            (:Completed
              (bind _array_element_6 (Utilities|Array|ForEachLoopwithBreak (Variables|Default|GetBackRights) :!label _label_6)
                (:LoopBody
                  (Utilities|CalculateValidMove _array_element_6
                    (:InValidMove
                      (goto _label_6 Break))
                    (:PieceToTake
                      (goto _label_6 Break))))
                (:Completed
                  (bind _array_element_7 (Utilities|Array|ForEachLoopwithBreak (Variables|Default|GetForwardLefts) :!label _label_7)
                    (:LoopBody
                      (Utilities|CalculateValidMove _array_element_7
                        (:InValidMove
                          (goto _label_7 Break))
                        (:PieceToTake
                          (goto _label_7 Break))))
                    (:Completed
                      (bind _array_element_8 (Utilities|Array|ForEachLoopwithBreak (Variables|Default|GetForwardRights) :!label _label_8)
                        (:LoopBody
                          (Utilities|CalculateValidMove _array_element_8
                            (:InValidMove
                              (goto _label_8 Break))
                            (:PieceToTake
                              (goto _label_8 Break))))))))))))))
    (:else)))

(event EventDeSelect
  (Rendering|Material|SetOverlayMaterial (Variables|Default|GetChessPiece) "/Game/Art/Materials/M_OutlineClear.M_OutlineClear" :!class /Script/Engine.MeshComponent)
  (for _array_element (Variables|Default|GetBackLefts)
    (Rendering|SetVisibility _array_element false false)
    (Collision|SetCollisionEnabled _array_element "NoCollision"))
  (for _array_element_2 (Variables|Default|GetBackRights)
    (Rendering|SetVisibility _array_element_2 false false)
    (Collision|SetCollisionEnabled _array_element_2 "NoCollision"))
  (for _array_element_3 (Variables|Default|GetForwardLefts)
    (Rendering|SetVisibility _array_element_3 false false)
    (Collision|SetCollisionEnabled _array_element_3 "NoCollision"))
  (for _array_element_4 (Variables|Default|GetForwardRights)
    (Rendering|SetVisibility _array_element_4 false false)
    (Collision|SetCollisionEnabled _array_element_4 "NoCollision")))

(event EventBeginPlay
  (bind _backlefts (Variables|Default|GetBackLefts))
  (bind _forwardrights (Variables|Default|GetForwardRights))
  (bind _forwardlefts (Variables|Default|GetForwardLefts))
  (bind _backrights (Variables|Default|GetBackRights))
  (|CallParentFunction)
  (Utilities|Array|Add _forwardrights (Variables|Default|GetForwardRight))
  (Utilities|Array|Add _forwardrights (Variables|Default|GetForwardRight1))
  (Utilities|Array|Add _forwardrights (Variables|Default|GetForwardRight2))
  (Utilities|Array|Add _forwardrights (Variables|Default|GetForwardRight3))
  (Utilities|Array|Add _forwardrights (Variables|Default|GetForwardRight4))
  (Utilities|Array|Add _forwardrights (Variables|Default|GetForwardRight5))
  (Utilities|Array|Add _forwardrights (Variables|Default|GetForwardRight6))
  (Utilities|Array|Add _forwardlefts (Variables|Default|GetForwardLeft))
  (Utilities|Array|Add _forwardlefts (Variables|Default|GetForwardLeft1))
  (Utilities|Array|Add _forwardlefts (Variables|Default|GetForwardLeft2))
  (Utilities|Array|Add _forwardlefts (Variables|Default|GetForwardLeft3))
  (Utilities|Array|Add _forwardlefts (Variables|Default|GetForwardLeft4))
  (Utilities|Array|Add _forwardlefts (Variables|Default|GetForwardLeft5))
  (Utilities|Array|Add _forwardlefts (Variables|Default|GetForwardLeft6))
  (Utilities|Array|Add _backrights (Variables|Default|GetBackRight))
  (Utilities|Array|Add _backrights (Variables|Default|GetBackRight1))
  (Utilities|Array|Add _backrights (Variables|Default|GetBackRight2))
  (Utilities|Array|Add _backrights (Variables|Default|GetBackRight3))
  (Utilities|Array|Add _backrights (Variables|Default|GetBackRight4))
  (Utilities|Array|Add _backrights (Variables|Default|GetBackRight5))
  (Utilities|Array|Add _backrights (Variables|Default|GetBackRight6))
  (Utilities|Array|Add _backlefts (Variables|Default|GetBackLeft))
  (Utilities|Array|Add _backlefts (Variables|Default|GetBackLeft1))
  (Utilities|Array|Add _backlefts (Variables|Default|GetBackLeft2))
  (Utilities|Array|Add _backlefts (Variables|Default|GetBackLeft3))
  (Utilities|Array|Add _backlefts (Variables|Default|GetBackLeft4))
  (Utilities|Array|Add _backlefts (Variables|Default|GetBackLeft5))
  (Utilities|Array|Add _backlefts (Variables|Default|GetBackLeft6)))

(fn ConstructionScript
  (|CallParentFunction))

(fn ReturnNumberOfValidMoves
  (bind _pieceking (Variables|Default|GetPieceKing)
    (:then
      (if (< (Utilities|Array|Length (Variables|/Game/Blueprints/Actors/BP_King.BP_King_C|GetPiecesCheckingKing _pieceking)) 2)
        (bind _array_element (Utilities|Array|ForEachLoopwithBreak (Variables|Default|GetBackLefts) :!label _label)
          (:LoopBody
            (Utilities|CalculateifPieceinPath _array_element (Utilities|Array|Get(acopy) (Variables|/Game/Blueprints/Actors/BP_King.BP_King_C|GetPiecesCheckingKing _pieceking))
              (:SpotClear
                _)
              (:PieceInTheWay
                (goto _label Break))
              (:EnemyToTakeFound
                _))
            (Utilities|CheckMoveCanBlockAttack (Utilities|Array|Get(acopy) (Variables|/Game/Blueprints/Actors/BP_King.BP_King_C|GetPiecesCheckingKing _pieceking)) _array_element
              (:CanBlock
                (LocalVariables|SetNumberOfValidMoves 1.0))))
          (:Completed
            (bind _array_element_2 (Utilities|Array|ForEachLoopwithBreak (Variables|Default|GetBackRights) :!label _label_2)
              (:LoopBody
                (Utilities|CalculateifPieceinPath _array_element_2 (Utilities|Array|Get(acopy) (Variables|/Game/Blueprints/Actors/BP_King.BP_King_C|GetPiecesCheckingKing _pieceking))
                  (:SpotClear
                    _)
                  (:PieceInTheWay
                    (goto _label_2 Break))
                  (:EnemyToTakeFound
                    _))
                (Utilities|CheckMoveCanBlockAttack (Utilities|Array|Get(acopy) (Variables|/Game/Blueprints/Actors/BP_King.BP_King_C|GetPiecesCheckingKing _pieceking)) _array_element_2
                  (:CanBlock
                    (LocalVariables|SetNumberOfValidMoves 1.0))))
              (:Completed
                (bind _array_element_3 (Utilities|Array|ForEachLoopwithBreak (Variables|Default|GetForwardLefts) :!label _label_3)
                  (:LoopBody
                    (Utilities|CalculateifPieceinPath _array_element_3 (Utilities|Array|Get(acopy) (Variables|/Game/Blueprints/Actors/BP_King.BP_King_C|GetPiecesCheckingKing _pieceking))
                      (:SpotClear
                        _)
                      (:PieceInTheWay
                        (goto _label_3 Break))
                      (:EnemyToTakeFound
                        _))
                    (Utilities|CheckMoveCanBlockAttack (Utilities|Array|Get(acopy) (Variables|/Game/Blueprints/Actors/BP_King.BP_King_C|GetPiecesCheckingKing _pieceking)) _array_element_3
                      (:CanBlock
                        (LocalVariables|SetNumberOfValidMoves 1.0))))
                  (:Completed
                    (bind _array_element_4 (Utilities|Array|ForEachLoopwithBreak (Variables|Default|GetForwardRights) :!label _label_4)
                      (:LoopBody
                        (Utilities|CalculateifPieceinPath _array_element_4 (Utilities|Array|Get(acopy) (Variables|/Game/Blueprints/Actors/BP_King.BP_King_C|GetPiecesCheckingKing _pieceking))
                          (:SpotClear
                            _)
                          (:PieceInTheWay
                            (goto _label_4 Break))
                          (:EnemyToTakeFound
                            _))
                        (Utilities|CheckMoveCanBlockAttack (Utilities|Array|Get(acopy) (Variables|/Game/Blueprints/Actors/BP_King.BP_King_C|GetPiecesCheckingKing _pieceking)) _array_element_4
                          (:CanBlock
                            (LocalVariables|SetNumberOfValidMoves 1.0)))))))))))
        (CallFunction|DeSelect :!label _label_5)
        (return (LocalVariables|GetNumberOfValidMoves))))
    (:else
      (goto _label_5))))