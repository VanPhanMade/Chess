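; Rook chess piece that shows its valid moves as square markers along four straight rays of seven.
; Each ray is walked outward, using line traces to find board and pieces, until blocked or an enemy can be taken.
; While its king is checked by one piece, it tests only for moves that block or take the attacker.
; ReturnNumberOfValidMoves flags whether any such check-answering move exists, and DeSelect hides the markers.
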(event EventDeSelect
  (Rendering|Material|SetOverlayMaterial (Variables|Default|GetChessPiece) "/Game/Art/Materials/M_OutlineClear.M_OutlineClear" :!class /Script/Engine.MeshComponent)
  (for _array_element (Variables|Default|GetForwards)
    (Collision|SetCollisionEnabled _array_element "NoCollision")
    (Rendering|SetVisibility _array_element false false))
  (for _array_element_2 (Variables|Default|GetBackwards)
    (Collision|SetCollisionEnabled _array_element_2 "NoCollision")
    (Rendering|SetVisibility _array_element_2 false false))
  (for _array_element_3 (Variables|Default|GetRights)
    (Collision|SetCollisionEnabled _array_element_3 "NoCollision")
    (Rendering|SetVisibility _array_element_3 false false))
  (for _array_element_4 (Variables|Default|GetLefts)
    (Collision|SetCollisionEnabled _array_element_4 "NoCollision")
    (Rendering|SetVisibility _array_element_4 false false)))

(event EventBeginPlay
  (bind _rights (Variables|Default|GetRights))
  (bind _backwards (Variables|Default|GetBackwards))
  (bind _lefts (Variables|Default|GetLefts))
  (bind _forwards (Variables|Default|GetForwards))
  (|CallParentFunction)
  (Utilities|Array|Add _forwards (Variables|Default|GetForward1))
  (Utilities|Array|Add _forwards (Variables|Default|GetForward2))
  (Utilities|Array|Add _forwards (Variables|Default|GetForward3))
  (Utilities|Array|Add _forwards (Variables|Default|GetForward4))
  (Utilities|Array|Add _forwards (Variables|Default|GetForward5))
  (Utilities|Array|Add _forwards (Variables|Default|GetForward6))
  (Utilities|Array|Add _forwards (Variables|Default|GetForward7))
  (Utilities|Array|Add _backwards (Variables|Default|GetBack1))
  (Utilities|Array|Add _backwards (Variables|Default|GetBack2))
  (Utilities|Array|Add _backwards (Variables|Default|GetBack3))
  (Utilities|Array|Add _backwards (Variables|Default|GetBack4))
  (Utilities|Array|Add _backwards (Variables|Default|GetBack5))
  (Utilities|Array|Add _backwards (Variables|Default|GetBack6))
  (Utilities|Array|Add _backwards (Variables|Default|GetBack7))
  (Utilities|Array|Add _rights (Variables|Default|GetRight1))
  (Utilities|Array|Add _rights (Variables|Default|GetRight2))
  (Utilities|Array|Add _rights (Variables|Default|GetRight3))
  (Utilities|Array|Add _rights (Variables|Default|GetRight4))
  (Utilities|Array|Add _rights (Variables|Default|GetRight5))
  (Utilities|Array|Add _rights (Variables|Default|GetRight6))
  (Utilities|Array|Add _rights (Variables|Default|GetRight7))
  (Utilities|Array|Add _lefts (Variables|Default|GetLeft1))
  (Utilities|Array|Add _lefts (Variables|Default|GetLeft2))
  (Utilities|Array|Add _lefts (Variables|Default|GetLeft3))
  (Utilities|Array|Add _lefts (Variables|Default|GetLeft4))
  (Utilities|Array|Add _lefts (Variables|Default|GetLeft5))
  (Utilities|Array|Add _lefts (Variables|Default|GetLeft6))
  (Utilities|Array|Add _lefts (Variables|Default|GetLeft7)))

(event EventShowValidMoves
  (bind _pieceking (Variables|Default|GetPieceKing)
    (:then
      (if (Variables|/Game/Blueprints/Actors/BP_King.BP_King_C|GetChecked _pieceking)
        (if (< (Utilities|Array|Length (Variables|/Game/Blueprints/Actors/BP_King.BP_King_C|GetPiecesCheckingKing _pieceking)) 2)
          (bind _array_element (Utilities|Array|ForEachLoopwithBreak (Variables|Default|GetForwards) :!label _label)
            (:LoopBody
              (Utilities|CalculateifPieceinPath _array_element (Utilities|Array|Get(acopy) (Variables|/Game/Blueprints/Actors/BP_King.BP_King_C|GetPiecesCheckingKing _pieceking))
                (:SpotClear
                  _)
                (:PieceInTheWay
                  (goto _label Break))
                (:EnemyToTakeFound
                  _))
              (Utilities|CheckMoveCanBlockAttack (Utilities|Array|Get(acopy) (Variables|/Game/Blueprints/Actors/BP_King.BP_King_C|GetPiecesCheckingKing _pieceking)) _array_element
                (:CanBlock
                  (goto _label Break))))
            (:Completed
              (bind _array_element_2 (Utilities|Array|ForEachLoopwithBreak (Variables|Default|GetBackwards) :!label _label_2)
                (:LoopBody
                  (Utilities|CalculateifPieceinPath _array_element_2 (Utilities|Array|Get(acopy) (Variables|/Game/Blueprints/Actors/BP_King.BP_King_C|GetPiecesCheckingKing _pieceking))
                    (:SpotClear
                      _)
                    (:PieceInTheWay
                      (goto _label_2 Break))
                    (:EnemyToTakeFound
                      _))
                  (Utilities|CheckMoveCanBlockAttack (Utilities|Array|Get(acopy) (Variables|/Game/Blueprints/Actors/BP_King.BP_King_C|GetPiecesCheckingKing _pieceking)) _array_element_2
                    (:CanBlock
                      (goto _label_2 Break))))
                (:Completed
                  (bind _array_element_3 (Utilities|Array|ForEachLoopwithBreak (Variables|Default|GetRights) :!label _label_3)
                    (:LoopBody
                      (Utilities|CalculateifPieceinPath _array_element_3 (Utilities|Array|Get(acopy) (Variables|/Game/Blueprints/Actors/BP_King.BP_King_C|GetPiecesCheckingKing _pieceking))
                        (:SpotClear
                          _)
                        (:PieceInTheWay
                          (goto _label_3 Break))
                        (:EnemyToTakeFound
                          _))
                      (Utilities|CheckMoveCanBlockAttack (Utilities|Array|Get(acopy) (Variables|/Game/Blueprints/Actors/BP_King.BP_King_C|GetPiecesCheckingKing _pieceking)) _array_element_3
                        (:CanBlock
                          (goto _label_3 Break))))
                    (:Completed
                      (bind _array_element_4 (Utilities|Array|ForEachLoopwithBreak (Variables|Default|GetLefts) :!label _label_4)
                        (:LoopBody
                          (Utilities|CalculateifPieceinPath _array_element_4 (Utilities|Array|Get(acopy) (Variables|/Game/Blueprints/Actors/BP_King.BP_King_C|GetPiecesCheckingKing _pieceking))
                            (:SpotClear
                              _)
                            (:PieceInTheWay
                              (goto _label_4 Break))
                            (:EnemyToTakeFound
                              _))
                          (Utilities|CheckMoveCanBlockAttack (Utilities|Array|Get(acopy) (Variables|/Game/Blueprints/Actors/BP_King.BP_King_C|GetPiecesCheckingKing _pieceking)) _array_element_4
                            (:CanBlock
                              (goto _label_4 Break))))))))))))
        (else
          (bind _array_element_5 (Utilities|Array|ForEachLoopwithBreak (Variables|Default|GetForwards) :!label _label_5)
            (:LoopBody
              (Utilities|CalculateValidMove _array_element_5
                (:InValidMove
                  (goto _label_5 Break))
                (:PieceToTake
                  (goto _label_5 Break))))
            (:Completed
              (bind _array_element_6 (Utilities|Array|ForEachLoopwithBreak (Variables|Default|GetBackwards) :!label _label_6)
                (:LoopBody
                  (Utilities|CalculateValidMove _array_element_6
                    (:InValidMove
                      (goto _label_6 Break))
                    (:PieceToTake
                      (goto _label_6 Break))))
                (:Completed
                  (bind _array_element_7 (Utilities|Array|ForEachLoopwithBreak (Variables|Default|GetRights) :!label _label_7)
                    (:LoopBody
                      (Utilities|CalculateValidMove _array_element_7
                        (:InValidMove
                          (goto _label_7 Break))
                        (:PieceToTake
                          (goto _label_7 Break))))
                    (:Completed
                      (bind _array_element_8 (Utilities|Array|ForEachLoopwithBreak (Variables|Default|GetLefts) :!label _label_8)
                        (:LoopBody
                          (Utilities|CalculateValidMove _array_element_8
                            (:InValidMove
                              (goto _label_8 Break))
                            (:PieceToTake
                              (goto _label_8 Break))))))))))))))
    (:else)))

(fn ConstructionScript
  (|CallParentFunction))

(fn ReturnNumberOfValidMoves
  (bind _pieceking (Variables|Default|GetPieceKing)
    (:then
      (if (< (Utilities|Array|Length (Variables|/Game/Blueprints/Actors/BP_King.BP_King_C|GetPiecesCheckingKing _pieceking)) 2)
        (bind _array_element (Utilities|Array|ForEachLoopwithBreak (Variables|Default|GetForwards) :!label _label)
          (:LoopBody
            (Utilities|CalculateifPieceinPath _array_element (Utilities|Array|Get(acopy) (Variables|/Game/Blueprints/Actors/BP_King.BP_King_C|GetPiecesCheckingKing _pieceking))
              (:SpotClear
                _)
              (:PieceInTheWay
                (goto _label Break))
              (:EnemyToTakeFound
                _))
            (Utilities|CheckMoveCanBlockAttack (Utilities|Array|Get(acopy) (Variables|/Game/Blueprints/Actors/BP_King.BP_King_C|GetPiecesCheckingKing _pieceking)) _array_element
              (:CanBlock
                (LocalVariables|SetValidMoves 1.0 :!label _label_2))))
          (:Completed
            (bind _array_element_2 (Utilities|Array|ForEachLoopwithBreak (Variables|Default|GetBackwards) :!label _label_3)
              (:LoopBody
                (Utilities|CalculateifPieceinPath _array_element_2 (Utilities|Array|Get(acopy) (Variables|/Game/Blueprints/Actors/BP_King.BP_King_C|GetPiecesCheckingKing _pieceking))
                  (:SpotClear
                    _)
                  (:PieceInTheWay
                    (goto _label_3 Break))
                  (:EnemyToTakeFound
                    _))
                (Utilities|CheckMoveCanBlockAttack (Utilities|Array|Get(acopy) (Variables|/Game/Blueprints/Actors/BP_King.BP_King_C|GetPiecesCheckingKing _pieceking)) _array_element_2
                  (:CanBlock
                    (goto _label_2))))
              (:Completed
                (bind _array_element_3 (Utilities|Array|ForEachLoopwithBreak (Variables|Default|GetRights) :!label _label_4)
                  (:LoopBody
                    (Utilities|CalculateifPieceinPath _array_element_3 (Utilities|Array|Get(acopy) (Variables|/Game/Blueprints/Actors/BP_King.BP_King_C|GetPiecesCheckingKing _pieceking))
                      (:SpotClear
                        _)
                      (:PieceInTheWay
                        (goto _label_4 Break))
                      (:EnemyToTakeFound
                        _))
                    (Utilities|CheckMoveCanBlockAttack (Utilities|Array|Get(acopy) (Variables|/Game/Blueprints/Actors/BP_King.BP_King_C|GetPiecesCheckingKing _pieceking)) _array_element_3
                      (:CanBlock
                        (goto _label_2))))
                  (:Completed
                    (bind _array_element_4 (Utilities|Array|ForEachLoopwithBreak (Variables|Default|GetLefts) :!label _label_5)
                      (:LoopBody
                        (Utilities|CalculateifPieceinPath _array_element_4 (Utilities|Array|Get(acopy) (Variables|/Game/Blueprints/Actors/BP_King.BP_King_C|GetPiecesCheckingKing _pieceking))
                          (:SpotClear
                            _)
                          (:PieceInTheWay
                            (goto _label_5 Break))
                          (:EnemyToTakeFound
                            _))
                        (Utilities|CheckMoveCanBlockAttack (Utilities|Array|Get(acopy) (Variables|/Game/Blueprints/Actors/BP_King.BP_King_C|GetPiecesCheckingKing _pieceking)) _array_element_4
                          (:CanBlock
                            (goto _label_2))))
                      (:Completed
                        _))))))))
        (CallFunction|DeSelect)
        (return (LocalVariables|GetValidMoves))))
    (:else
      (return (LocalVariables|GetValidMoves)))))